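; BP_Wapple is a customizable Swapple character that dresses itself from the saved appearance in the SV_SwappleChar slot.
; On BeginPlay or ReloadSaveState, it sets the BodyColor material parameter on every skeletal mesh and assigns saved static meshes to the equipment components, mirroring hands and shoes.
; A saved hat replaces hair on the shared Hair component.
; SaveSkin passes the current color to the game instance.
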(event `SaveSkin`
  (bind _asswapple_game_instance (cast `/Game/_Main/SwappleGameInstance` (`GameplayStatics.GetGameInstance`)))
  (`/Game/_Main/SwappleGameInstance.SetColor` _asswapple_game_instance (`self.Color`)))

(event `ReloadSaveState`
  (bind _returnvalue (`GameplayStatics.LoadGameFromSlot` "SV_SwappleChar" :!label _label))
  (bind _assv_swapple (cast `/Game/_Main/SV_Swapple` _returnvalue))
  (for _array_element (`self.K2_GetComponentsByClass` "/Script/Engine.SkeletalMeshComponent")
    (bind (_hat _facial _accessories _shirt _hands _pants _shoes _color _hair) (break `/Game/_Main/Structures/S_Equipped` (`/Game/_Main/SV_Swapple.Equips` _assv_swapple)))
    (`MeshComponent.SetVectorParameterValueOnMaterials` _array_element "BodyColor" (`KismetMathLibrary.Conv_LinearColorToVector` _color)))
  (set `self.Color` _color)
  (`StaticMeshComponent.SetStaticMesh` (`self.Hair`) (select `bool` (== _hat null) :`false` _hat :`true` _hair))
  (`StaticMeshComponent.SetStaticMesh` (`self.Facial`) _facial)
  (`StaticMeshComponent.SetStaticMesh` (`self.Accessories`) _accessories)
  (`StaticMeshComponent.SetStaticMesh` (`self.Shirt`) _shirt)
  (`StaticMeshComponent.SetStaticMesh` (`self.HandR`) _hands)
  (`StaticMeshComponent.SetStaticMesh` (`self.HandL`) _hands)
  (`StaticMeshComponent.SetStaticMesh` (`self.Pants`) _pants)
  (`StaticMeshComponent.SetStaticMesh` (`self.ShoesR`) _shoes)
  (`StaticMeshComponent.SetStaticMesh` (`self.ShoesL`) _shoes))

(event `self.ReceiveBeginPlay`
  (goto _label))

(fn `UserConstructionScript`)