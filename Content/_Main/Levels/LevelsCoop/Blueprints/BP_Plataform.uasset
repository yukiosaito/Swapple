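; BP_Plataform is a platform actor for the co-op levels that moves vertically when triggered.
; Each call to its Active event toggles IsUp, playing the timeline when up and reversing it when down.
; The timeline curve, scaled by Height, offsets the actor's Z from the location cached in the Construction Script.
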(event `self.Active`
  (bind (_vectorlocation_x _vectorlocation_y _vectorlocation_z) (`KismetMathLibrary.BreakVector` (`self.VectorLocation`)))
  (set `self.IsUp` (not (`self.IsUp`)))
  (if (`self.IsUp`)
    (bind (_direction _height) (`Timeline|Timeline_0` :!label _label)
      (:`Update`
        (`self.K2_SetActorLocation` (`KismetMathLibrary.MakeVector` _vectorlocation_x _vectorlocation_y (+ (* _height (`self.Height`)) _vectorlocation_z)))))
    (else
      (goto _label :!via `Reverse`))))

(fn `UserConstructionScript`
  (`parent.UserConstructionScript`)
  (set `self.VectorLocation` (`self.K2_GetActorLocation`)))