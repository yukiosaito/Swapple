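; Player pawn for a co-op level whose movement inputs and eight skill keys resolve through remappable order arrays, recording used bindings as known.
; Skills come from the GameState and trigger Interact or Die via S_ then M_ events, blocking actions meanwhile.
; Interact calls an overlapping BP_MasterInteract; Die teleports the pawn to the "Die"-tagged PlayerStart after a delay.
; The construction script applies body color and cosmetic meshes from the GameInstance's Equips.
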(event `Skill`
  (params (Index :type Integer))
  (bind _knownskill (`self.KnownSkill`))
  (bind _output (`|GetArrayItem` (`self.KeyOrderSkill`) Index))
  (if (not (`self.BlockActions`))
    (switch `string` _output
      (:`Interact`
        (`KismetArrayLibrary.Array_Set` _knownskill Index _output)
        (`self.S_Interagir`))
      (:`Die`
        (`KismetArrayLibrary.Array_Set` _knownskill Index _output)
        (`self.S_Die`)))))

(event `self.ReceiveBeginPlay`
  (bind _asgame_state_level_coop (cast `/Game/_Main/Levels/LevelsCoop/GameStateLevelCoop` (`GameplayStatics.GetGameState`)))
  (bind _output_get (set `self.KeyOrderSkill` (`/Game/_Main/Levels/LevelsCoop/GameStateLevelCoop.Skills` _asgame_state_level_coop)))
  (set `self.KnownSkill` _output_get))

(event `S_Interagir`
  (set `self.BlockActions` true)
  (set `self.AnimationString` "Interagir")
  (`self.M_Interagir`))

(event `KeyMovement`
  (params (ItemToFind :type "Key Structure (by ref)"))
  (bind _knownmov (`self.KnownMov`))
  (bind _returnvalue (`KismetMathLibrary.MakeRotator` 0.0 0.0 (.yaw (`self.GetControlRotation`))))
  (bind (_returnvalue_x _returnvalue_y _returnvalue_z) (`KismetMathLibrary.BreakVector` (`KismetMathLibrary.GetForwardVector` _returnvalue)))
  (bind (_returnvalue_x_2 _returnvalue_y_2 _returnvalue_z_2) (`KismetMathLibrary.BreakVector` (`KismetMathLibrary.GetRightVector` _returnvalue)))
  ;[0.00014 1 0] Movement
  (if (not (`self.BlockActions`))
    (switch `int` (`KismetArrayLibrary.Array_Find` (`self.KeyOrderMov`) ItemToFind)
      (:`0`
        (`KismetArrayLibrary.Array_Set` _knownmov 0 true)
        (`self.AddMovementInput` (`KismetMathLibrary.MakeVector` 0.0 _returnvalue_y_2 _returnvalue_z_2) -1.0))
      (:`1`
        (`KismetArrayLibrary.Array_Set` _knownmov 1 true)
        (`self.AddMovementInput` (`KismetMathLibrary.MakeVector` _returnvalue_x 0.0 _returnvalue_z)))
      (:`2`
        (`KismetArrayLibrary.Array_Set` _knownmov 2 true)
        (`self.AddMovementInput` (`KismetMathLibrary.MakeVector` 0.0 _returnvalue_y_2 _returnvalue_z_2)))
      (:`3`
        (`KismetArrayLibrary.Array_Set` _knownmov 3 true)
        (`self.AddMovementInput` (`KismetMathLibrary.MakeVector` _returnvalue_x 0.0 _returnvalue_z) -1.0)))))

(event `M_Interagir`
  (bind _asbp_master_interact (cast `/Game/_Main/Levels/LevelsCoop/Blueprints/BP_MasterInteract` (`|GetArrayItem` (`PrimitiveComponent.GetOverlappingActors` (`self.CapsuleComponent`) "/Game/_Main/Levels/LevelsCoop/Blueprints/BP_MasterInteract.BP_MasterInteract_C")))
    (:`then`
      (`/Game/_Main/Levels/LevelsCoop/Blueprints/BP_MasterInteract.Interagir` _asbp_master_interact))
    (:`CastFailed`
      _))
  (`KismetSystemLibrary.Delay` 0.2)
  (set `self.BlockActions` false)
  (set `self.AnimationString` ""))

(event `InputAxis|MoveForward`
  (params (AxisValue :type "Float (single-precision)"))
  ;[0.00014 1 0] Movement
  (switch `int` (`KismetMathLibrary.FTrunc` AxisValue)
    (:`-1`
      (`self.KeyMovement` (`self.DownRef`)))
    (:`1`
      (`self.KeyMovement` (`self.UpRef`)))))

(event `S_Die`
  (set `self.BlockActions` true)
  (set `self.AnimationString` "Die")
  (`self.M_Die`))

(event `InputAxis|MoveRight`
  (params (AxisValue :type "Float (single-precision)"))
  ;[0.00014 1 0] Movement
  (switch `int` (`KismetMathLibrary.FTrunc` AxisValue)
    (:`-1`
      (`self.KeyMovement` (`self.LeftRef`)))
    (:`1`
      (`self.KeyMovement` (`self.RightRef`)))))

(event `M_Die`
  (`KismetSystemLibrary.Delay` 3.0)
  (bind _outactors (`GameplayStatics.GetAllActorsOfClassWithTag` "/Script/Engine.PlayerStart" "Die"))
  (`self.K2_SetActorTransform` (`self.GetTransform` (`|GetArrayItem` _outactors)) false true)
  (`KismetSystemLibrary.Delay` 0.1)
  (set `self.BlockActions` false)
  (set `self.AnimationString` ""))

(event `InputAction|Hab1`
  (params (Key :type "Key Structure"))
  (:`Pressed`
    (`self.Skill` 0)))

(event `InputAction|Hab2`
  (params (Key :type "Key Structure"))
  (:`Pressed`
    (`self.Skill` 1)))

(event `InputAction|Hab3`
  (params (Key :type "Key Structure"))
  (:`Pressed`
    (`self.Skill` 2)))

(event `InputAction|Hab4`
  (params (Key :type "Key Structure"))
  (:`Pressed`
    (`self.Skill` 3)))

(event `InputAction|Hab5`
  (params (Key :type "Key Structure"))
  (:`Pressed`
    (`self.Skill` 4)))

(event `InputAction|Hab6`
  (params (Key :type "Key Structure"))
  (:`Pressed`
    (`self.Skill` 5)))

(event `InputAction|Hab7`
  (params (Key :type "Key Structure"))
  (:`Pressed`
    (`self.Skill` 6)))

(event `InputAction|Hab8`
  (params (Key :type "Key Structure"))
  (:`Pressed`
    (`self.Skill` 7)))

(fn `UserConstructionScript`
  (locals (Equips :type "/Game/_Main/Structures/S_Equipped Structure"))
  (bind (_hat _facial _accessories _shirt _hands _pants _shoes _color _hair) (break `/Game/_Main/Structures/S_Equipped` (`local.Equips`)))
  (bind _asswapple_game_instance (cast `/Game/_Main/SwappleGameInstance` (`GameplayStatics.GetGameInstance`)))
  (bind _output_get (set `local.Equips` (`/Game/_Main/SwappleGameInstance.Equips` _asswapple_game_instance)))
  (for _array_element (`self.K2_GetComponentsByClass` "/Script/Engine.SkeletalMeshComponent")
    (`MeshComponent.SetVectorParameterValueOnMaterials` _array_element "BodyColor" (`KismetMathLibrary.Conv_LinearColorToVector` (`.Color_17_FFF8FB1A406AF5C7D1DB32BFA55B30F3` (break `/Game/_Main/Structures/S_Equipped` _output_get)))))
  (`StaticMeshComponent.SetStaticMesh` (`self.Hair`) (select `bool` (== _hat null) :`false` _hat :`true` _hair))
  (`StaticMeshComponent.SetStaticMesh` (`self.Facial`) _facial)
  (`StaticMeshComponent.SetStaticMesh` (`self.Accessories`) _accessories)
  (`StaticMeshComponent.SetStaticMesh` (`self.Shirt`) _shirt)
  (`StaticMeshComponent.SetStaticMesh` (`self.Pants`) _pants)
  (`StaticMeshComponent.SetStaticMesh` (`self.ShoesR`) _shoes)
  (`StaticMeshComponent.SetStaticMesh` (`self.ShoesL`) _shoes)
  (`StaticMeshComponent.SetStaticMesh` (`self.ShirtR`) _hands)
  (`StaticMeshComponent.SetStaticMesh` (`self.ShirtL`) _hands))